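; Beam actor that kills an Enemy1 caught between it and a beam target actor.
; Every Tick it sphere-traces from its own location to the first "target"-tagged Beam_target_Blueprint.
; If the hit component is the capsule of an Enemy1, found through a lookup with tag None, it sets IsDead and destroys that enemy.
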(event `self.ReceiveTick`
  (params (DeltaSeconds :type "Float (single-precision)"))
  (bind _outactors (`GameplayStatics.GetAllActorsWithTag` "target"))
  (bind _asbeam_target_blueprint (cast `/Game/Beam_target_Blueprint` (`|GetArrayItem` _outactors)))
  (bind (_outhit _returnvalue) (`KismetSystemLibrary.SphereTraceSingle` (`self.K2_GetActorLocation`) (`self.K2_GetActorLocation` _asbeam_target_blueprint) 25.0 "TraceTypeQuery3" false (`|MakeArray` null :!type "Actor Object Reference")))
  (bind _outactors_2 (`GameplayStatics.GetAllActorsWithTag` "None"))
  (bind _asenemy_1 (cast `/Game/SideScrollerBP/Blueprints/Enemy1` (`|GetArrayItem` _outactors_2)))
  (if _returnvalue
    (if (== (`.HitComponent` (`GameplayStatics.BreakHitResult` _outhit)) (`|GetArrayItem` (`self.GetComponentsByTag` _asenemy_1 "/Script/Engine.CapsuleComponent" "None")))
      (set `self.isDead` true)
      (`self.K2_DestroyActor` _asenemy_1))))

(fn `UserConstructionScript`
  (`parent.UserConstructionScript`))