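; Double-candle child Blueprint that adds a second flame, with its own point light, spot light, particle and smoke mesh, to the parent candle.
; Each overridden event calls the parent, then mirrors flicker, on/off switching and color lerping onto the second flame's components.
; The construction script presets the lit or unlit state and creates a dynamic smoke material, which cooling randomizes along with mesh scale and the smoke update fades through opacity.
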(event `self.ReceiveBeginPlay`
  (bind _particlesystem (`self.ParticleSystem`))
  ;[1 1 1] Begin play particle safety
  (`parent.ReceiveBeginPlay`)
  (`SceneComponent.SetVisibility` _particlesystem true false)
  (`ActorComponent.SetActive` _particlesystem (`self.LightOn`) false))

(event `self.CandleLight__UpdateFunc`
  ;[1 1 1] Second light flicker
  (`parent.CandleLight__UpdateFunc`)
  (`LightComponent.SetIntensity` (`self.PointLight1`) (* (`self.CandleLightValue`) (`self.LightIntencity`))))

(event `self.CandleOn`
  (bind _flamecolor (`self.FlameColor`))
  (bind _pointlight1 (`self.PointLight1`))
  (bind _spotlight1 (`self.SpotLight1`))
  (bind _particlesystem (`self.ParticleSystem`))
  ;[1 1 1] Ingame turning on
  (`parent.CandleOn`)
  (`LightComponent.SetIntensity` _pointlight1 (`self.LightIntencity`))
  (`PointLightComponent.SetAttenuationRadius` _pointlight1 (`self.AttenuationRadius`))
  (`LightComponentBase.SetCastShadows` _pointlight1 (`self.LightShadows`))
  (`LightComponent.SetLightColor` _pointlight1 _flamecolor true)
  (`LightComponent.SetLightColor` _spotlight1 _flamecolor true)
  (`LightComponent.SetIntensity` _spotlight1 (`self.SSLight`))
  (`LightComponentBase.SetCastShadows` _spotlight1 (`self.LightShadows`))
  (`ParticleSystemComponent.SetColorParameter` _particlesystem "Color" _flamecolor)
  (`SceneComponent.SetHiddenInGame` _particlesystem false false)
  (`ActorComponent.SetActive` _particlesystem true true))

(event `self.CandleOff`
  (params (Cooling :type Boolean) (Smoke :type Boolean))
  ;[1 1 1] Ingame turning off
  (`parent.CandleOff` Cooling Smoke)
  (`LightComponent.SetIntensity` (`self.PointLight1`) 0.0)
  (`LightComponent.SetIntensity` (`self.SpotLight1`) 0.0)
  (`SceneComponent.SetHiddenInGame` (`self.ParticleSystem`) true false))

(event `self.ColorChange__UpdateFunc`
  (bind _returnvalue (`KismetMathLibrary.LinearColorLerp` (`self.FlameColor`) (`self.TempColor`) (`self.ColorLerp`)))
  ;[1 1 1] Lerp light color
  (`parent.ColorChange__UpdateFunc`)
  (`LightComponent.SetLightColor` (`self.PointLight1`) _returnvalue true)
  (`LightComponent.SetLightColor` (`self.SpotLight1`) _returnvalue true)
  (`ParticleSystemComponent.SetColorParameter` (`self.ParticleSystem`) "Color" _returnvalue))

(event `self.Cooling`
  (bind _returnvalue (`KismetMathLibrary.RandomFloatInRange` 0.3 1.0))
  (bind _smokemat2 (`self.SmokeMat2`))
  ;[1 1 1] Randomize smoke
  (`parent.Cooling`)
  (`MaterialInstanceDynamic.SetScalarParameterValue` _smokemat2 "R" (`KismetMathLibrary.RandomFloatInRange` 0.0 1.0))
  (`MaterialInstanceDynamic.SetScalarParameterValue` _smokemat2 "G" (`KismetMathLibrary.RandomFloatInRange` 0.0 1.0))
  (`MaterialInstanceDynamic.SetScalarParameterValue` _smokemat2 "G" (`KismetMathLibrary.RandomFloatInRange` 0.0 1.0))
  (`MaterialInstanceDynamic.SetScalarParameterValue` _smokemat2 "B-A" (`KismetMathLibrary.RandomFloatInRange` 0.0 1.0))
  (`SceneComponent.SetWorldScale3D` (`self.StaticMesh`) (`KismetMathLibrary.MakeVector` _returnvalue _returnvalue _returnvalue)))

(event `self.SmokeTilemine__UpdateFunc`
  (bind _smokemat2 (`self.SmokeMat2`))
  ;[1 1 1] Candle smoke
  (`parent.SmokeTilemine__UpdateFunc`)
  (if (`self.Smoke`)
    (`MaterialInstanceDynamic.SetScalarParameterValue` _smokemat2 "OpacityTop" (`KismetMathLibrary.Lerp` -1.0 1.0 (`self.SmokeOnLerp`)))
    (`MaterialInstanceDynamic.SetScalarParameterValue` _smokemat2 "OpacityBot" (`KismetMathLibrary.Lerp` 1.0 -1.0 (`self.SmokeOffLerp`)))))

(fn `UserConstructionScript`
  (bind _flamecolor (`self.FlameColor`))
  (bind _pointlight1 (`self.PointLight1`))
  (bind _spotlight1 (`self.SpotLight1`))
  (bind _particlesystem (`self.ParticleSystem`))
  (bind _staticmesh (`self.StaticMesh`))
  (`parent.UserConstructionScript`)
  ;[1 1 1] Creating dynamic material instance
  (bind _returnvalue (`PrimitiveComponent.CreateDynamicMaterialInstance` _staticmesh 0 (`PrimitiveComponent.GetMaterial` _staticmesh 0)))
  (set `self.SmokeMat2` _returnvalue)
  (`MaterialInstanceDynamic.SetScalarParameterValue` (`self.SmokeMat2`) "OpacityTop" 1.0)
  ;[1 1 1] Flame-light On/Off
  (if (`self.LightOn`)
    ;[1 1 1] Sets particle and light values
    (`LightComponent.SetIntensity` _pointlight1 (`self.LightIntencity`))
    (`PointLightComponent.SetAttenuationRadius` _pointlight1 (`self.AttenuationRadius`))
    (`LightComponentBase.SetCastShadows` _pointlight1 (`self.LightShadows`))
    (`LightComponent.SetLightColor` _pointlight1 _flamecolor true)
    (`LightComponent.SetLightColor` _spotlight1 _flamecolor true)
    (`LightComponent.SetIntensity` _spotlight1 (`self.SSLight`))
    (`ParticleSystemComponent.SetColorParameter` _particlesystem "Color" _flamecolor)
    (`SceneComponent.SetVisibility` _particlesystem true false)
    (else
      ;[1 1 1] set light intensity to 0 and decibels particles
      (`LightComponent.SetIntensity` (`self.PointLight1`) 0.0)
      (`LightComponent.SetIntensity` (`self.SpotLight1`) 0.0)
      (`SceneComponent.SetVisibility` (`self.ParticleSystem`) false false))))