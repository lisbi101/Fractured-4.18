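; Candle actor with flame particle, point and spot lights, wick glow and smoke mesh, switchable on and off in game.
; Construction script creates dynamic materials, applies colors and light settings, and randomizes flame distortion per instance.
; A looping CandleLight timeline drives point light intensity, with an occasional random flicker after a random loop count.
; CandleOn, CandleOff and ChangeColor control it at runtime, using timelines for wick cooling, randomized smoke and color blending.
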(event `self.ReceiveBeginPlay`
  (bind _p_plomienswieczki2 (`self.P_plomienSwieczki2`))
  (bind _lighton (`self.LightOn`))
  ;[1 1 1] Safety for candle on/off
  (set `self.LightLoop_Flicker` (`KismetMathLibrary.RandomIntegerInRange` 10 50))
  (`SceneComponent.SetVisibility` _p_plomienswieczki2 true true)
  (`ActorComponent.SetActive` _p_plomienswieczki2 _lighton true)
  (if _lighton
    ;[1 1 1] Randomize start of light flickering
    (`KismetSystemLibrary.Delay` (`KismetMathLibrary.RandomFloatInRange` 0.0 0.5))
    ;[1 1 1] Light flickering
    (bind (_direction _lightintencity _flicker) (`Timeline|CandleLight` :!via `PlayFromStart` :!label _label)
      (:`Update`
        (if (== (`self.LightLoop`) (`self.LightLoop_Flicker`))
          (set `self.Flicker` _flicker)
          (if (`self.RandomFlicker`)
            (`ParticleSystemComponent.SetFloatParameter` (`self.P_plomienSwieczki2`) "Opacity" (`KismetMathLibrary.Lerp` -1.0 1.0 _flicker))
            (`LightComponent.SetIntensity` (`self.PointLight`) (`KismetMathLibrary.Lerp` (`self.LightIntencity`) 0.0 _flicker)))
          (if (`KismetMathLibrary.NearlyEqual_FloatFloat` (`self.Flicker`) 0.0 0.001)
            (set `self.RandomFlicker` (`KismetMathLibrary.RandomBool`)))
          (else
            (set `self.CandleLightValue` _lightintencity)
            (`LightComponent.SetIntensity` (`self.PointLight`) (* _lightintencity (`self.LightIntencity`))))))
      (:`End`
        (`TimelineComponent.SetPlayRate` (`self.CandleLight`) (`KismetMathLibrary.RandomFloatInRange` 0.8 1.2))
        (if (== (`self.LightLoop`) (`self.LightLoop_Flicker`))
          (set `self.LightLoop` 0)
          (set `self.LightLoop_Flicker` (`KismetMathLibrary.RandomIntegerInRange` 10 50))
          (`ParticleSystemComponent.SetFloatParameter` (`self.P_plomienSwieczki2`) "Opacity" -1.0)
          (set `self.Flicker` 0.0)
          (else
            (`/Engine/EditorBlueprintResources/StandardMacros.IncrementInt` (`self.LightLoop`))))))
    (else
      (`self.CandleOff` false false))))

(event `CandleOff`
  (params (Cooling :type Boolean :default true) (Smoke :type Boolean :default true))
  ;[1 1 1] Ingame turning off
  (set `self.Smoke` Smoke)
  (`LightComponent.SetIntensity` (`self.PointLight`) 0.0)
  (`LightComponent.SetIntensity` (`self.SpotLight`) 0.0)
  (if Cooling
    (`self.Cooling`)
    (goto _label :!via `Stop`)
    (else
      (`SceneComponent.SetHiddenInGame` (`self.P_plomienSwieczki2`) true false)
      (`MaterialInstanceDynamic.SetScalarParameterValue` (`self.CandleMaterial`) "candlewick_brightness" 0.0)
      (goto _label :!via `Stop`))))

(event `CandleOn`
  (bind _flamecolor (`self.FlameColor`))
  (bind _spotlight (`self.SpotLight`))
  (bind _p_plomienswieczki2 (`self.P_plomienSwieczki2`))
  (bind _pointlight (`self.PointLight`))
  (bind _smokemat (`self.SmokeMat`))
  ;[1 1 1] Ingame turning on
  (`self.StopCooling`)
  (`self.StopSmoke`)
  (`LightComponent.SetIntensity` _pointlight (`self.LightIntencity`))
  (`PointLightComponent.SetAttenuationRadius` _pointlight (`self.AttenuationRadius`))
  (`LightComponentBase.SetCastShadows` _pointlight (`self.LightShadows`))
  (`LightComponent.SetLightColor` _pointlight _flamecolor true)
  (`LightComponent.SetLightColor` _spotlight _flamecolor true)
  (`LightComponent.SetIntensity` _spotlight (`self.SSLight`))
  (`LightComponent.SetIntensity` _spotlight (`self.SSLight`))
  (`LightComponentBase.SetCastShadows` _spotlight (`self.LightShadows`))
  (`ParticleSystemComponent.SetColorParameter` _p_plomienswieczki2 "Color" _flamecolor)
  (`ParticleSystemComponent.SetFloatParameter` _p_plomienswieczki2 "Opacity" -1.0)
  (`SceneComponent.SetHiddenInGame` _p_plomienswieczki2 false false)
  (`ActorComponent.SetActive` _p_plomienswieczki2 true true)
  (`MaterialInstanceDynamic.SetScalarParameterValue` (`self.CandleMaterial`) "candlewick_brightness" 2.0)
  (`MaterialInstanceDynamic.SetScalarParameterValue` _smokemat "OpacityTop" 1.0)
  (`MaterialInstanceDynamic.SetScalarParameterValue` _smokemat "OpacityBot" -1.0)
  (goto _label :!via `PlayFromStart`))

(event `ChangeColor`
  (params (NewColot :type "LinearColor Structure") (`InterpSpeed(S)` :type "Float (double-precision)" :default 1.0))
  ;[1 1 1] Lerp light color
  (set `self.TempColor` NewColot)
  (`TimelineComponent.SetPlayRate` (`self.ColorChange`) `InterpSpeed(S)`)
  (bind (_direction _lerp) (`Timeline|ColorChange` :!via `PlayFromStart`)
    (:`Update`
      (set `self.ColorLerp` _lerp)
      (bind _returnvalue (`KismetMathLibrary.LinearColorLerp` (`self.FlameColor`) (`self.TempColor`) _lerp))
      (`LightComponent.SetLightColor` (`self.PointLight`) _returnvalue true)
      (`LightComponent.SetLightColor` (`self.SpotLight`) _returnvalue true)
      (`ParticleSystemComponent.SetColorParameter` (`self.P_plomienSwieczki2`) "Color" _returnvalue))
    (:`Finished`
      (set `self.FlameColor` (`self.TempColor`)))))

(event `Cooling`
  (bind _returnvalue (`KismetMathLibrary.RandomFloatInRange` 0.3 1.0))
  (bind _smokemat (`self.SmokeMat`))
  (bind _smokemat_2 (`self.SmokeMat`))
  ;[1 1 1] Off anim
  (`|ExecutionSequence`
    (:`then_0`
      ;[1 1 1] candle wick "cooling"
      (bind (_direction _lerp _firelerp) (`Timeline|CandleWickCooling` :!via `PlayFromStart` :!label _label_2)
        (:`Update`
          (`MaterialInstanceDynamic.SetScalarParameterValue` (`self.CandleMaterial`) "candlewick_brightness" (`KismetMathLibrary.Lerp` 0.0 2.0 _lerp))
          (`ParticleSystemComponent.SetFloatParameter` (`self.P_plomienSwieczki2`) "Opacity" (`KismetMathLibrary.Lerp` 1.0 -1.0 _firelerp)))
        (:`Finished`
          (`SceneComponent.SetHiddenInGame` (`self.P_plomienSwieczki2`) true false))))
    (:`then_1`
      ;[1 1 1] Candle smoke
      (if (`self.Smoke`)
        ;;[1 1 1] Randomize smoke
        (`MaterialInstanceDynamic.SetScalarParameterValue` _smokemat_2 "R" (`KismetMathLibrary.RandomFloatInRange` 0.0 1.0))
        (`MaterialInstanceDynamic.SetScalarParameterValue` _smokemat_2 "G" (`KismetMathLibrary.RandomFloatInRange` 0.0 1.0))
        (`MaterialInstanceDynamic.SetScalarParameterValue` _smokemat_2 "B-A" (`KismetMathLibrary.RandomFloatInRange` 0.0 1.0))
        (`SceneComponent.SetWorldScale3D` (`self.SM_smoke`) (`KismetMathLibrary.MakeVector` _returnvalue _returnvalue _returnvalue))
        (`TimelineComponent.SetPlayRate` (`self.SmokeTilemine`) (`KismetMathLibrary.RandomFloatInRange` (`self.SmokeFadeSpeedMin`) (`self.SmokeFadeSpeedMax`)))
        (bind (_direction_2 _smokeon _smokeoff) (`Timeline|SmokeTilemine` :!via `PlayFromStart` :!label _label_3)
          (:`Update`
            (set `self.SmokeOnLerp` _smokeon)
            (set `self.SmokeOffLerp` _smokeoff)
            (`MaterialInstanceDynamic.SetScalarParameterValue` _smokemat "OpacityTop" (`KismetMathLibrary.Lerp` -1.0 1.0 _smokeon))
            (`MaterialInstanceDynamic.SetScalarParameterValue` _smokemat "OpacityBot" (`KismetMathLibrary.Lerp` 1.0 -1.0 _smokeoff)))
          (:`PlayRateSwap`
            (`TimelineComponent.SetPlayRate` (`self.SmokeTilemine`) (`KismetMathLibrary.RandomFloatInRange` (`self.SmokeFadeSpeedMin`) (`self.SmokeFadeSpeedMax`)))))))))

(event `StopCooling`
  (goto _label_2 :!via `Stop`))

(event `StopSmoke`
  ;[1 1 1] Candle smoke
  (goto _label_3 :!via `Stop`))

(fn `UserConstructionScript`
  (bind _candlematerial (`self.CandleMaterial`))
  (bind _pointlight (`self.PointLight`))
  (bind _p_plomienswieczki2 (`self.P_plomienSwieczki2`))
  (bind _spotlight (`self.SpotLight`))
  (bind _flamecolor (`self.FlameColor`))
  (bind _candlematerial_2 (`self.CandleMaterial`))
  (bind _particlematerial (`self.ParticleMaterial`))
  (bind _sm_candle (`self.SM_Candle`))
  (bind _sm_smoke (`self.SM_smoke`))
  ;[1 1 1] Creating dynamic material instance
  (bind _returnvalue (`PrimitiveComponent.CreateDynamicMaterialInstance` _sm_smoke 0 (`PrimitiveComponent.GetMaterial` _sm_smoke 0)))
  (set `self.SmokeMat` _returnvalue)
  (`MaterialInstanceDynamic.SetScalarParameterValue` (`self.SmokeMat`) "OpacityTop" 1.0)
  (bind _returnvalue_2 (`PrimitiveComponent.CreateDynamicMaterialInstance` _sm_candle 0 (`PrimitiveComponent.GetMaterial` _sm_candle 0)))
  (set `self.CandleMaterial` _returnvalue_2)
  (`PrimitiveComponent.SetMaterial` _sm_candle (`self.Lod1Mat`) _candlematerial)
  (`PrimitiveComponent.SetMaterial` _sm_candle (`self.Lod2Mat`) _candlematerial)
  (`MaterialInstanceDynamic.SetVectorParameterValue` _candlematerial_2 "Color" (`self.CandleColor`))
  (`MaterialInstanceDynamic.SetVectorParameterValue` _candlematerial_2 "SSS_Color" (`self.CandleSSSColor`))
  (bind _returnvalue_3 (`PrimitiveComponent.CreateDynamicMaterialInstance` (`self.P_plomienSwieczki2`) 0 "/Game/AtmosphericCandlesPack/Materials/MP_CandleFlame_Inst.MP_CandleFlame_Inst"))
  (set `self.ParticleMaterial` _returnvalue_3)
  ;[1 1 1] Randomizes flame material values
  (bind _returnvalue_4 (`MaterialInstanceDynamic.K2_GetScalarParameterValue` _particlematerial "DistortionSpeed"))
  (`MaterialInstanceDynamic.SetScalarParameterValue` _particlematerial "DistortionSpeed" (+ _returnvalue_4 (`KismetMathLibrary.RandomFloatInRange` -0.2 0.2)))
  (bind _returnvalue_5 (`MaterialInstanceDynamic.K2_GetScalarParameterValue` _particlematerial "DistortionLengh"))
  (`MaterialInstanceDynamic.SetScalarParameterValue` _particlematerial "DistortionLengh" (+ _returnvalue_5 (`KismetMathLibrary.RandomFloatInRange` -1.0 2.0)))
  (bind _returnvalue_6 (`MaterialInstanceDynamic.K2_GetScalarParameterValue` _particlematerial "FlameMoveSpeed"))
  (`MaterialInstanceDynamic.SetScalarParameterValue` _particlematerial "FlameMoveSpeed" (+ _returnvalue_6 (`KismetMathLibrary.RandomFloatInRange` -0.2 0.2)))
  (bind _returnvalue_7 (`MaterialInstanceDynamic.K2_GetVectorParameterValue` _particlematerial "DistortionIntencity"))
  (bind (_r _g _b) (break `LinearColor` _returnvalue_7))
  (`MaterialInstanceDynamic.SetVectorParameterValue` _particlematerial "DistortionIntencity" (make `LinearColor` (+ _r (`KismetMathLibrary.RandomFloatInRange` -0.02 0.02)) (+ _g (`KismetMathLibrary.RandomFloatInRange` -0.02 0.02)) (+ _b (`KismetMathLibrary.RandomFloatInRange` -0.02 0.02))))
  ;[1 1 1] Flame-light On/Off
  (if (`self.LightOn`)
    ;[1 1 1] Sets particle and light values
    (`LightComponent.SetIntensity` _pointlight (`self.LightIntencity`))
    (`PointLightComponent.SetAttenuationRadius` _pointlight (`self.AttenuationRadius`))
    (`LightComponentBase.SetCastShadows` _pointlight (`self.LightShadows`))
    (`LightComponent.SetLightColor` _pointlight _flamecolor true)
    (`LightComponent.SetLightColor` _spotlight _flamecolor true)
    (`LightComponent.SetIntensity` _spotlight (`self.SSLight`))
    (`LightComponent.SetIntensity` _spotlight (`self.SSLight`))
    (`ParticleSystemComponent.SetColorParameter` _p_plomienswieczki2 "Color" _flamecolor)
    (`SceneComponent.SetVisibility` _p_plomienswieczki2 true false)
    (`MaterialInstanceDynamic.SetScalarParameterValue` (`self.CandleMaterial`) "candlewick_brightness" 2.0)
    (else
      ;[1 1 1] set light intensity to 0 and decibels particles
      (`LightComponent.SetIntensity` (`self.PointLight`) 0.0)
      (`LightComponent.SetIntensity` (`self.SpotLight`) 0.0)
      (`MaterialInstanceDynamic.SetScalarParameterValue` (`self.CandleMaterial`) "candlewick_brightness" 0.0)
      (`SceneComponent.SetVisibility` (`self.P_plomienSwieczki2`) false false))))